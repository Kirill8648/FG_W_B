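; Game mode for the fast rolling-ball variant that keeps respawning the player's ball whenever it is destroyed.
; On BeginPlay it casts the player pawn to PhysicsBallBP, overrides its jump impulse and binds to its destroyed event.
; After destruction and a short delay, it spawns a PhysicsBallBPFast at RespawnLocation, possesses it and calls Respawn to repeat that setup on the new ball.
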(event Custom|OnDestroyed_
  (params (DestroyedActor :type Actor%20Object%20Reference))
  (Utilities|FlowControl|Delay 2.0)
  (bind _returnvalue (Game|SpawnActorfromClass "/Game/BluePrint/PhysicsBallBPFast.PhysicsBallBPFast_C" (Variables|Default|GetRespawnLocation) "AlwaysSpawn" 0 0))
  (Pawn|Possess (Game|GetPlayerController 0) _returnvalue)
  (CallFunction|Respawn))

(event Custom|Respawn
  (bind _asphysics_ball_bp (Utilities|Casting|CastToPhysicsBallBP (Game|Player|GetPlayerPawn 0)))
  (Variables|/Game/BluePrint/PhysicsBallBP.PhysicsBallBP_C|SetJumpImpulse _asphysics_ball_bp 1e+07)
  (Game|BindEventtoOnDestroyed _asphysics_ball_bp (delegate Custom|OnDestroyed_)))

(event EventBeginPlay
  (bind _asphysics_ball_bp (Utilities|Casting|CastToPhysicsBallBP (Game|Player|GetPlayerPawn 0)))
  (Variables|/Game/BluePrint/PhysicsBallBP.PhysicsBallBP_C|SetJumpImpulse _asphysics_ball_bp 1e+07)
  (Game|BindEventtoOnDestroyed _asphysics_ball_bp (delegate Custom|OnDestroyed_)))

(fn ConstructionScript)