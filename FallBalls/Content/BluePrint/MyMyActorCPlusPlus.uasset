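; Debug test actor that visualises vector rotation math around a hard-coded line segment, apparently groundwork for placing Bezier control points.
; A Box overlap prints the segment's Y and Z angles, draws it, then plays a timeline whose angle feeds RingRotateVector to plot a trail of points.
; The construction script runs a static version of the same drawing.
; Helper functions derive signed angles and a control point, but the Bezier drawing chains are disconnected.
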(event OnComponentBeginOverlap(Box)
  (params (OverlappedComponent :type Primitive%20Component%20Object%20Reference) (OtherActor :type Actor%20Object%20Reference) (OtherComp :type Primitive%20Component%20Object%20Reference) (OtherBodyIndex :type Integer) (bFromSweep :type Boolean) (SweepResult :type Hit%20Result%20Structure%20%28by%20ref%29))
  (bind _returnvalue (Math|Vector|MakeVector 0.0 0.0 0.0))
  (bind _returnvalue_2 (Math|Vector|MakeVector 3e+02 4e+02 0.0))
  (bind _z (Variables|Default|GetZ))
  (Development|PrintString (Utilities|String|ToString(Float) (CallFunction|AnglVectorZ _returnvalue _returnvalue_2)))
  (Development|PrintString (Utilities|String|ToString(Float) (CallFunction|AnglVectorY _returnvalue _returnvalue_2)))
  (Rendering|Debug|DrawDebugLine _returnvalue _returnvalue_2 "(R=0.055785,G=0.609375,B=0.000000,A=1.000000)" 5.0 0.0)
  (Rendering|Debug|DrawDebugPoint _returnvalue 1e+01 "(R=0.358212,G=1.000000,B=0.859512,A=1.000000)" 5.0)
  (Rendering|Debug|DrawDebugPoint _returnvalue_2 1e+01 "(R=0.463769,G=1.000000,B=0.930153,A=1.000000)" 5.0)
  (Rendering|Debug|DrawDebugPoint (Class|MyActorCPlusPlus|RingRotateVector _returnvalue _returnvalue_2 1e+02 0.0 _z 0.0 0.0) 2e+01 "(R=1.000000,G=0.895246,B=0.000000,A=1.000000)" 5.0)
  (bind _angle (Timeline|Timeline_1 PlayFromStart)
    (:Update
      (Rendering|Debug|DrawDebugPoint (Class|MyActorCPlusPlus|RingRotateVector _returnvalue _returnvalue_2 1e+02 _angle _z 0.0 0.0) 1e+01 "(R=1.000000,G=0.030746,B=0.060593,A=1.000000)" 5.0))))

(event EventBeginPlay)

(event Collision|EventActorBeginOverlap
  (params (OtherActor :type Actor%20Object%20Reference)))

(event EventTick
  (params (DeltaSeconds :type Float%20%28single-precision%29)))

(fn ConstructionScript
  (bind _returnvalue (Math|Vector|MakeVector 0.0 0.0 0.0))
  (bind _returnvalue_2 (Math|Vector|MakeVector 3e+02 4e+02 0.0))
  (Development|PrintString (Utilities|String|ToString(Float) (CallFunction|AnglVectorZ _returnvalue _returnvalue_2)))
  (Development|PrintString (Utilities|String|ToString(Float) (CallFunction|AnglVectorY _returnvalue _returnvalue_2)))
  (Rendering|Debug|DrawDebugLine _returnvalue _returnvalue_2 "(R=0.055785,G=0.609375,B=0.000000,A=1.000000)" 5.0 0.0)
  (Rendering|Debug|DrawDebugPoint _returnvalue 1e+01 "(R=0.358212,G=1.000000,B=0.859512,A=1.000000)" 5.0)
  (Rendering|Debug|DrawDebugPoint _returnvalue_2 1e+01 "(R=0.463769,G=1.000000,B=0.930153,A=1.000000)" 5.0)
  (Rendering|Debug|DrawDebugPoint "0, 0, 0" 2e+01 "(R=1.000000,G=0.895246,B=0.000000,A=1.000000)" 5.0)
  (Rendering|Debug|DrawDebugPoint (Class|MyActorCPlusPlus|RingRotateVector _returnvalue _returnvalue_2 1e+02 0.0 0.0 0.0 0.0) 1e+01 "(R=1.000000,G=0.030746,B=0.060593,A=1.000000)" 5.0))

(fn GetControlPointforBezierCurve
  (params (A :type Vector) (B :type Vector) (BC :type Float%20%28single-precision%29) (Angle :type Float%20%28single-precision%29) (Distance :type Float%20%28single-precision%29))
  (return (Class|MyActorCPlusPlus|RingRotateVector A B 1e+02 Angle (CallFunction|AnglVectorY A B) 0.0 Distance)))

(fn AnglVectorY
  (params (Begin :type Vector) (End :type Vector))
  (bind _returnvalue (- End Begin))
  (bind (_x _y _z) (Math|Vector|BreakVector _returnvalue))
  (bind _returnvalue_2 (Math|Vector|MakeVector _y _x 0.0))
  (bind _returnvalue_3 (Class|KismetMathLibrary|VectorCosineAngle2D _returnvalue_2 "0,1.000000, 0"))
  (bind _returnvalue_4 (Class|KismetMathLibrary|DegAcos _returnvalue_3))
  (if (> (.Y (Math|Vector|BreakVector Begin)) (.Y (Math|Vector|BreakVector End)))
    (return _returnvalue_4)
    (else
      (return (* _returnvalue_4 -1.0)))))

(fn AnglVectorZ
  (params (Begin :type Vector) (End :type Vector))
  (bind _returnvalue (- End Begin))
  (bind (_x _y _z) (Math|Vector|BreakVector _returnvalue))
  (bind _returnvalue_2 (Math|Vector|MakeVector _y _z 0.0))
  (bind _returnvalue_3 (Class|KismetMathLibrary|VectorCosineAngle2D _returnvalue_2 "0,1.000000, 0"))
  (bind _returnvalue_4 (Class|KismetMathLibrary|DegAcos _returnvalue_3))
  (if (> (.Z (Math|Vector|BreakVector End)) (.Z (Math|Vector|BreakVector Begin)))
    (return (* _returnvalue_4 -1.0))
    (else
      (return _returnvalue_4))))