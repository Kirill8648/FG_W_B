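; Game mode for a rolling-ball game that keeps a minutes and seconds timer and respawns the player's ball.
; While IsCount is true, Tick uses a one-second Delay to advance Seconds and roll it over into Minutes.
; BeginPlay binds to the player ball's OnDestroyed event.
; On destruction it waits briefly, spawns a new PhysicsBallBP at RespawnLocation, possesses it and rebinds through Respawn.
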(event Custom|OnDestroyed_
  (params (DestroyedActor :type Actor%20Object%20Reference))
  (Utilities|FlowControl|Delay 2.0)
  (bind _returnvalue (Game|SpawnActorfromClass "/Game/BluePrint/PhysicsBallBP.PhysicsBallBP_C" (Variables|Default|GetRespawnLocation) "AlwaysSpawn" 0 0))
  (Pawn|Possess (Game|GetPlayerController 0) _returnvalue)
  (CallFunction|Respawn))

(event Custom|Respawn
  (bind _asphysics_ball_bp (Utilities|Casting|CastToPhysicsBallBP (Game|Player|GetPlayerPawn 0)))
  (Game|BindEventtoOnDestroyed _asphysics_ball_bp (delegate Custom|OnDestroyed_)))

(event EventBeginPlay
  (bind _asphysics_ball_bp (Utilities|Casting|CastToPhysicsBallBP (Game|Player|GetPlayerPawn 0)))
  (Game|BindEventtoOnDestroyed _asphysics_ball_bp (delegate Custom|OnDestroyed_)))

(event EventTick
  (params (DeltaSeconds :type Float%20%28single-precision%29))
  (if (Variables|Default|GetIsCount?)
    (Utilities|FlowControl|Delay 1.0)
    (Variables|Default|SetSeconds (+ (Variables|Default|GetSeconds) 1))
    (if (> (Variables|Default|GetSeconds) 59)
      (Variables|Default|SetMinutes (+ (Variables|Default|GetMinutes) 1))
      (Variables|Default|SetSeconds 0))))

(fn ConstructionScript)