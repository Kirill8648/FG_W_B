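; Debug test actor that moves a cube around an axis running from its root to a SetEnd offset, apparently tracing a ring.
; After a one-second delay, BeginPlay draws the axis, then the Angle timeline feeds an external RotateVector helper to position the cube and plot its path.
; Angle3d builds that helper's AxisZ direction from SetEnd's planar cosine angles.
; Angle2d, Bezier and construction-script experiments are left unconnected.
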(event EventBeginPlay
  (bind _defaultsceneroot (Variables|Default|GetDefaultSceneRoot))
  (bind _returnvalue (Transformation|GetWorldLocation _defaultsceneroot))
  (Utilities|FlowControl|Delay 1.0)
  (Variables|Default|Setstart _returnvalue)
  (Variables|Default|Setend (+ _returnvalue (Variables|Default|Getset%20end)))
  (Development|PrintString (Utilities|String|ToString(Vector) (CallFunction|Angle3d (Variables|Default|Getset%20end))))
  (Rendering|Debug|DrawDebugLine (Variables|Default|Getstart) (Variables|Default|Getend) "(R=0.055785,G=0.609375,B=0.000000,A=1.000000)" 2e+01 0.0)
  (Rendering|Debug|DrawDebugPoint (Variables|Default|Getstart) 1e+01 "(R=0.358212,G=1.000000,B=0.859512,A=1.000000)" 2e+01)
  (Rendering|Debug|DrawDebugPoint (Variables|Default|Getend) 1e+01 "(R=0.463769,G=1.000000,B=0.930153,A=1.000000)" 2e+01)
  (bind _angle (Timeline|Angle Play)
    (:Update
      (Rendering|Debug|DrawDebugPoint (Class|RingVector|RotateVector (Variables|Default|Getstart) (Variables|Default|Getend) (Variables|Default|GetBC) _angle (Variables|Default|GetDistance) (Math|Vector|Normalize (Variables|Default|Getset%20end) 1.0) (CallFunction|Angle3d (Variables|Default|Getset%20end))) 1e+01 "(R=1.000000,G=0.030746,B=0.060593,A=1.000000)" 2e+01)
      (Transformation|SetWorldLocation (Variables|Default|GetCube) (Class|RingVector|RotateVector (Variables|Default|Getstart) (Variables|Default|Getend) (Variables|Default|GetBC) _angle (Variables|Default|GetDistance) (Math|Vector|Normalize (Variables|Default|Getset%20end) 1.0) (CallFunction|Angle3d (Variables|Default|Getset%20end))) false false))))

(event Collision|EventActorBeginOverlap
  (params (OtherActor :type Actor%20Object%20Reference)))

(event EventTick
  (params (DeltaSeconds :type Float%20%28single-precision%29)))

(fn ConstructionScript)

(fn Angle2d
  (params (vector :type Vector))
  (bind (_x _y) (Math|Vector|BreakVector vector))
  (bind _returnvalue (Math|Vector|MakeVector _x _y 0.0))
  (bind _returnvalue_2 (Class|KismetMathLibrary|VectorCosineAngle2D _returnvalue "1.000000,0.000000,0.000000"))
  (bind _returnvalue_3 (Class|KismetMathLibrary|DegAcos _returnvalue_2))
  (bind _returnvalue_4 (Math|Rotator|MakeRotator 0.0 0.0 _returnvalue_3))
  (bind _returnvalue_5 (Math|Vector|RotateVector "1.000000, 0,0.000000" _returnvalue_4))
  (bind (_x_2 _y_2) (Math|Vector|BreakVector _returnvalue_5))
  (if (< (.Y (Math|Vector|BreakVector vector)) 0.0)
    (return (Math|Vector|MakeVector _x_2 (* _y_2 -1.0) 0.0))
    (else
      (return _returnvalue_5))))

(fn Angle3d
  (params (Vector :type Vector))
  (bind (_x _y _z) (Math|Vector|BreakVector Vector))
  (bind (_x_2 _y_2) (Math|Vector|BreakVector Vector))
  (bind _returnvalue (Math|Vector|MakeVector _x _z 0.0))
  (bind _returnvalue_2 (Math|Vector|MakeVector _x_2 _y_2 0.0))
  (bind _returnvalue_3 (Class|KismetMathLibrary|VectorCosineAngle2D _returnvalue "0.000000,1.000000,0.000000"))
  (bind _returnvalue_4 (Class|KismetMathLibrary|VectorCosineAngle2D _returnvalue_2 "1.000000,0.000000,0.000000"))
  (bind _returnvalue_5 (Class|KismetMathLibrary|DegAcos _returnvalue_3))
  (bind _returnvalue_6 (Class|KismetMathLibrary|DegAcos _returnvalue_4))
  (bind _returnvalue_7 (* _returnvalue_5 -1.0))
  (bind _returnvalue_8 (Math|Rotator|MakeRotator 0.0 _returnvalue_7 _returnvalue_6))
  (bind _returnvalue_9 (Math|Vector|RotateVector "1.000000, 0,0.000000" _returnvalue_8))
  (if (< (.Y (Math|Vector|BreakVector Vector)) 0.0)
    (return _returnvalue_9)
    (else
      (return _returnvalue_9))))